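; Music visualizer actor that makes a set of skull actors glow and emit particles in response to musical notes.
; On BeginPlay it gives each skull's static mesh its own dynamic material instance.
; Each tick, the matching note amplitude from MusicParticles drives that skull's emission hue and brightness through HSV mapping.
; The note spawn delegate places particles at a local offset from a skull chosen by wrapping the note index.
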(event SpawnParticleDelegate(MusicParticles)
  (params (noteIndex :type Integer))
  (bind _skulls (Variables|Default|GetSkulls))
  (Class|MusicParticles1|SpawnParticleforNote (Variables|Default|GetMusicParticles) noteIndex (Math|Transform|TransformLocation (Transformation|GetActorTransform (Utilities|Array|Get(acopy) _skulls (Math|Integer|%(Integer) noteIndex (Utilities|Array|Length _skulls)))) "150.000000,0.000000,150.000000") "/Game/ParticleSystems/ParticleSystem2.ParticleSystem2"))

(event EventBeginPlay
  (for _array_element (Variables|Default|GetSkulls)
    (bind _returnvalue (Rendering|Material|CreateDynamicMaterialInstance "/Game/PaigeAssets/SkullMaterial.SkullMaterial" "None" "None" :!class /Script/Engine.KismetMaterialLibrary))
    (Rendering|Material|SetMaterial (Actor|GetComponentbyClass _array_element "/Script/Engine.StaticMeshComponent") 0 _returnvalue)
    (Utilities|Array|Add (Variables|Default|GetMaterialInterfaces) _returnvalue)))

(event EventTick
  (params (DeltaSeconds :type Float%20%28single-precision%29))
  (for (_array_element _array_index) (Variables|Default|GetMaterialInterfaces)
    (Rendering|Material|SetVectorParameterValue _array_element "emission" (Class|KismetMathLibrary|HSVtoRGB (Math|Float|MapRangeClamped (Math|Float|Sqrt (Utilities|Array|Get(acopy) (Variables|/Script/MLTest2.MusicParticles1|GetNoteAmplitudes (Variables|Default|GetMusicParticles)) _array_index)) 0.2 0.6 0.0 2e+02) 1.0 (Math|Float|MapRangeClamped (Utilities|Array|Get(acopy) (Variables|/Script/MLTest2.MusicParticles1|GetNoteAmplitudes (Variables|Default|GetMusicParticles)) _array_index) 0.0 0.06 0.0 0.4) 1.0) :!class /Script/Engine.MaterialInstanceDynamic)))

(fn ConstructionScript)