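; Game mode for a multi-user Pictures at Exhibition experience that assigns player starts by role: server view, VR or AR.
; ChoosePlayerStart gives the local controller the first ServerView start.
; Remote players get a free VR start if GetPlatformName, evaluated on the machine running the game mode, returns Windows, otherwise an AR (Lumin) start.
; Claimed VR/AR starts have PlayerStartTag set to Taken, and debug prints report branches and failures.
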(event EventBeginPlay)

(event EventTick
  (params (DeltaSeconds :type Float%20%28single-precision%29)))

(fn ConstructionScript)

(fn ChoosePlayerStart
  (params (Player :type Controller%20Object%20Reference))
  (if (Pawn|IsLocalPlayerController Player)
    (Development|PrintString "Is Server" true true "(R=0.000000,G=0.660000,B=1.000000,A=1.000000)" 1e+01)
    ;[1 1 1] Choose Available Server Spawn Location
    (bind _outactors (Actor|GetAllActorsOfClasswithTag "/Script/Engine.PlayerStart" "ServerView"))
    (if (>= (Utilities|Array|Length _outactors) 1)
      (Development|PrintString "Successfully Got Server Pawn")
      (return (Utilities|Array|Get(acopy) _outactors))
      (else
        (Development|PrintString "ERROR: Server failed to Spawn Pawn")))
    (else
      (Development|PrintString "Is Client" true true "(R=0.000000,G=0.660000,B=1.000000,A=1.000000)" 1e+01)
      (if (Utilities|Enum|Equal(Enum) "Windows" (Game|GetPlatformName))
        (Development|PrintString "Is Windows" true true "(R=0.000000,G=0.660000,B=1.000000,A=1.000000)" 1e+01)
        ;[1 1 1] Choose Available VR Spawn Location
        (bind _outactors_2 (Actor|GetAllActorsOfClasswithTag "/Script/Engine.PlayerStart" "VR"))
        (for _array_element _outactors_2
          (if (Utilities|Name|NotEqual(Name) (Variables|/Script/Engine.PlayerStart|GetPlayerStartTag _array_element) "Taken")
            (Variables|/Script/Engine.PlayerStart|SetPlayerStartTag _array_element "Taken")
            (return _array_element)))
        (Development|PrintString "ERROR: No More Free VR Spots")
        (else
          (Development|PrintString "Is Lumin" true true "(R=0.000000,G=0.660000,B=1.000000,A=1.000000)" 1e+01)
          ;[1 1 1] Choose Available AR Spawn Location
          (bind _outactors_3 (Actor|GetAllActorsOfClasswithTag "/Script/Engine.PlayerStart" "AR"))
          (for _array_element_2 _outactors_3
            (if (Utilities|Name|NotEqual(Name) (Variables|/Script/Engine.PlayerStart|GetPlayerStartTag _array_element_2) "Taken")
              (Variables|/Script/Engine.PlayerStart|SetPlayerStartTag _array_element_2 "Taken")
              (return _array_element_2)))
          (Development|PrintString "ERROR: No More Free AR Spots"))))))