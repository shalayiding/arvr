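; XR player pawn that syncs its camera's transform from the owning player to peers.
; After setup on BeginPlay, the locally controlled pawn gathers rep-transform structs on Tick, relative to XRTransform, and passes them through SendRepToServer.
; Non-local copies interpolate components toward TargetReps, with relative, world and forced-reattach modes.
; On non-Windows remote clients it also unhides VR-tagged actors, despite a comment saying it hides them for AR.
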(event EventBeginPlay
  (Utilities|FlowControl|Sequence
    (:then_0
      (Utilities|FlowControl|Delay 0.1)
      (CallFunction|FreshSpawn))
    (:then_1
      ;[1 1 1] Hide All VR Actors If AR
      (Networking|SwitchHasAuthority
        (:Remote
          (if (Utilities|Enum|NotEqual(Enum) (Game|GetPlatformName) "Windows")
            (bind _outactors (Actor|GetAllActorswithTag "VR"))
            (for _array_element _outactors
              (Rendering|SetActorHiddenInGame _array_element false))))))))

(event Collision|EventActorBeginOverlap
  (params (OtherActor :type Actor%20Object%20Reference)))

(event EventTick
  (params (DeltaSeconds :type Float%20%28single-precision%29))
  (if (Pawn|IsLocallyControlled)
    (if (Variables|Default|GetInit%20Done)
      (Utilities|FlowControl|Sequence
        (:then_1
          (CallFunction|TickOwnerBeginRepliacte))))
    (else
      (CallFunction|TickPeerApplyRep))))

(event Custom|FreshSpawn
  (Utilities|FlowControl|Sequence
    (:then_0
      (CallFunction|StartAllSetupReplicate))
    (:then_1
      (Variables|Default|SetInit%20Done true))))

(event Custom|Start%20All%20Setup%20Replicate
  (CallFunction|InitReplicationSetup))

(event Custom|Tick%20Owner%20Begin%20Repliacte
  (Utilities|RateLimiter 0.0
    (:Out
      (bind _torep (CallFunction|GatherRepTransform (Variables|Default|GetToRep)))
      (bind _output_get (Variables|Default|SetToRep _torep))
      (CallFunction|SendReptoServer _output_get))))

(event Custom|Send%20Rep%20To%20Server
  (params (Target%20Reps :type Array%20of%20Rep%20Transform%20Structures))
  (Variables|Default|SetTarget%20Reps Target%20Reps))

(event Custom|Tick%20Peer%20Apply%20Rep
  (CallFunction|ApplyRepTransform (Variables|Default|GetTarget%20Reps)))

(fn ConstructionScript)

(fn InitReplicationSetup
  (Variables|Default|SetToRep (Utilities|Array|MakeArray (Utilities|Struct|MakeRepTransform (Variables|Default|GetXR_Camera) "0.000000,0.000000,0.000000|0.000000,0.000000,0.000000|1.000000,1.000000,1.000000" true false (Variables|Default|GetXR_Transform)))))

(fn GatherRepTransform
  (params (Array :type Array%20of%20Rep%20Transform%20Structures))
  (for _array_element Array
    (if (.Rel? (Utilities|Struct|BreakRepTransform _array_element))
      (if (== (Transformation|GetAttachParent (.TargetScene (Utilities|Struct|BreakRepTransform _array_element))) (.Parent (Utilities|Struct|BreakRepTransform _array_element)))
        (Utilities|Array|AddUnique (LocalVariables|GetNewReps) (Utilities|Struct|MakeRepTransform (.TargetScene (Utilities|Struct|BreakRepTransform _array_element)) (Transformation|GetWorldTransform (.TargetScene (Utilities|Struct|BreakRepTransform _array_element))) (.Rel? (Utilities|Struct|BreakRepTransform _array_element)) (.ForceRel (Utilities|Struct|BreakRepTransform _array_element)) (Transformation|GetAttachParent (.TargetScene (Utilities|Struct|BreakRepTransform _array_element))) (Transformation|GetRelativeTransform (.TargetScene (Utilities|Struct|BreakRepTransform _array_element))) (.Skip (Utilities|Struct|BreakRepTransform _array_element))) :!label _label)
        (else
          (Utilities|Array|AddUnique (LocalVariables|GetNewReps) (Utilities|Struct|MakeRepTransform (.TargetScene (Utilities|Struct|BreakRepTransform _array_element)) (.NewWorldTransform (Utilities|Struct|BreakRepTransform _array_element)) (.Rel? (Utilities|Struct|BreakRepTransform _array_element)) (.ForceRel (Utilities|Struct|BreakRepTransform _array_element)) (.Parent (Utilities|Struct|BreakRepTransform _array_element)) (Math|Transform|MakeRelativeTransform (Transformation|GetWorldTransform (.TargetScene (Utilities|Struct|BreakRepTransform _array_element))) (Transformation|GetWorldTransform (.Parent (Utilities|Struct|BreakRepTransform _array_element)))) (.Skip (Utilities|Struct|BreakRepTransform _array_element))))))
      (else
        (goto _label))))
  (return (LocalVariables|GetNewReps)))

(fn ApplyRepTransform
  (params (Array :type Array%20of%20Rep%20Transform%20Structures))
  (bind _returnvalue (Utilities|Time|GetWorldDeltaSeconds))
  (for _array_element Array
    (if (not (.Skip (Utilities|Struct|BreakRepTransform _array_element)))
      (if (.Rel? (Utilities|Struct|BreakRepTransform _array_element))
        (if (== (Transformation|GetAttachParent (.TargetScene (Utilities|Struct|BreakRepTransform _array_element))) (.Parent (Utilities|Struct|BreakRepTransform _array_element)))
          (Transformation|SetRelativeTransform (.TargetScene (Utilities|Struct|BreakRepTransform _array_element)) (Class|KismetMathLibrary|TInterpto (Transformation|GetRelativeTransform (.TargetScene (Utilities|Struct|BreakRepTransform _array_element))) (.RelativeTransform (Utilities|Struct|BreakRepTransform _array_element)) _returnvalue 7.0) false false :!label _label))
        (elif (.ForceRel (Utilities|Struct|BreakRepTransform _array_element))
          (Transformation|AttachComponentToComponent (.TargetScene (Utilities|Struct|BreakRepTransform _array_element)) (.Parent (Utilities|Struct|BreakRepTransform _array_element)) "None" "SnapToTarget" "KeepRelative" "KeepRelative" true)
          (goto _label)
          (else
            (Transformation|SetWorldTransform (.TargetScene (Utilities|Struct|BreakRepTransform _array_element)) (Class|KismetMathLibrary|TInterpto (Transformation|GetWorldTransform (.TargetScene (Utilities|Struct|BreakRepTransform _array_element))) (.NewWorldTransform (Utilities|Struct|BreakRepTransform _array_element)) _returnvalue 7.0) false false))))))
  (return))