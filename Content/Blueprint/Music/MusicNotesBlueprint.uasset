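; Actor that spawns music note particle effects in response to note events from its MusicParticles component.
; The component's spawn delegate passes a note index, which goes back into SpawnParticleForNote with the music notes particle template.
; Each effect appears at a random point in a flat vertical box, transformed from actor space to world space.
; A grid mapping from note index to location exists in NoteIndexToLocation but is unused.
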(event SpawnParticleDelegate(MusicParticles)
  (params (noteIndex :type Integer))
  (Class|MusicParticles1|SpawnParticleforNote (Variables|Default|GetMusicParticles) noteIndex (Math|Transform|TransformLocation (Transformation|GetActorTransform) (Math|Random|RandomPointinBoundingBox "0, 0, 0" "0.000000,150.000000,75.000000")) "/Game/ParticleSystems/ParticleSystemMusicNotes.ParticleSystemMusicNotes"))

(event EventBeginPlay)

(fn ConstructionScript)