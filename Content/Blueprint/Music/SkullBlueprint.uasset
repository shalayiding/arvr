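; Music visualizer actor that lights up 72 static meshes, one per note, using skull materials.
; BeginPlay spawns the meshes at NoteIndexToLocation positions, each with its own dynamic material.
; Every tick, MusicParticles note amplitudes drive each material's emission hue and brightness through HSV mapping.
; The MusicParticles spawn delegate emits skull particles at the triggering note's position, transformed by the actor.
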(event SpawnParticleDelegate(MusicParticles)
  (params (noteIndex :type Integer))
  (Class|MusicParticles1|SpawnParticleforNote (Variables|Default|GetMusicParticles) noteIndex (Math|Transform|TransformLocation (Transformation|GetActorTransform) (Utilities|NoteIndextoLocation noteIndex)) "/Game/ParticleSystems/ParticleSystemSkulls.ParticleSystemSkulls"))

(event EventBeginPlay
  (for _index (range 0 71)
    (bind _returnvalue (AddComponent|AddStaticMeshComponent false (Math|Transform|MakeTransform (Utilities|NoteIndextoLocation _index) "0, 0, 0" "0.100000,0.100000,0.100000")))
    (bind _returnvalue_2 (Rendering|Material|CreateDynamicMaterialInstance "/Game/Materials/SkullMaterialOld.SkullMaterialOld" "None" "None" :!class /Script/Engine.KismetMaterialLibrary))
    (Rendering|Material|SetMaterial _returnvalue 0 _returnvalue_2)
    (Utilities|Array|Add (Variables|Default|GetMaterialInterfaces) _returnvalue_2)))

(event EventTick
  (params (DeltaSeconds :type Float%20%28single-precision%29))
  (for (_array_element _array_index) (Variables|Default|GetMaterialInterfaces)
    (Rendering|Material|SetVectorParameterValue _array_element "emission" (Class|KismetMathLibrary|HSVtoRGB (Math|Float|MapRangeClamped (Math|Float|Sqrt (Utilities|Array|Get(acopy) (Variables|/Script/MLTest2.MusicParticles1|GetNoteAmplitudes (Variables|Default|GetMusicParticles)) _array_index)) 0.2 0.6 0.0 2e+02) 1.0 (Math|Float|MapRangeClamped (Utilities|Array|Get(acopy) (Variables|/Script/MLTest2.MusicParticles1|GetNoteAmplitudes (Variables|Default|GetMusicParticles)) _array_index) 0.0 0.06 0.0 0.4) 1.0) :!class /Script/Engine.MaterialInstanceDynamic)))

(fn ConstructionScript)