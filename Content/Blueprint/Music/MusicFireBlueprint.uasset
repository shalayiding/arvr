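; Music-reactive fire Blueprint that drives a set of particle systems from note amplitudes.
; Each tick it splits the MusicParticles NoteAmplitudes array into equal bands, one per particle system.
; It takes the loudest note in each band and feeds it, scaled up, into that system's "amplitude" float parameter.
; A NoteIndexToLocation graph holds an unused grid-position calculation.
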(event EventBeginPlay)

(event EventTick
  (params (DeltaSeconds :type Float%20%28single-precision%29))
  (bind _particlesystems (Variables|Default|GetParticleSystems))
  (bind _musicparticles (Variables|Default|GetMusicParticles))
  (bind _returnvalue (Utilities|Array|Length _particlesystems))
  (bind _noteamplitudes (Variables|/Script/MLTest2.MusicParticles1|GetNoteAmplitudes _musicparticles))
  (bind _returnvalue_2 (Utilities|Array|Length _noteamplitudes))
  (bind _returnvalue_3 (/ _returnvalue_2 _returnvalue))
  (for (_array_element _array_index) _particlesystems
    (Variables|Default|SetMax 0.0)
    (for _index (range (* _returnvalue_3 _array_index) (- (* (+ _array_index 1) _returnvalue_3) 1))
      (Variables|Default|SetMax (Math|Float|Max(Float) (Variables|Default|GetMax) (Utilities|Array|Get(acopy) _noteamplitudes _index))))
    (Effects|Components|ParticleSystem|SetFloatParameter (Variables|/Script/Engine.Emitter|GetParticleSystemComponent _array_element) "amplitude" (* (Variables|Default|GetMax) 5.0))))

(fn ConstructionScript)