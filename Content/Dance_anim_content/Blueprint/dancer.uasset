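; Dancer actor that plays a selectable dance animation on its mesh and spawns the scene UI.
; On BeginPlay it creates the UI_scene widget, hands it a reference to itself, adds it to the viewport, then applies the initial dance.
; Both BeginPlay and the Changedance event pass the DanceType variable to ChangeMode on the mesh's Dance animation instance.
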(event Custom|Change%20dance
  ;[1 0.01984 0] EVENTS CALL
  ;[0.2608 1 0] Event to change dance
  (Default|ChangeMode (.AsDance (Utilities|Casting|CastToDance (Components|SkeletalMesh|GetAnimInstance (Variables|/Script/Engine.Character|GetMesh self)))) (Variables|Default|GetDance_type)))

(event EventBeginPlay
  ;[1 0.01984 0] EVENTS CALL
  (Utilities|FlowControl|Sequence
    (:then_0
      ;[0.4701 0.3537 1] create ui scene
      (bind _returnvalue (UserInterface|CreateWidget "/Game/Dance_anim_content/Blueprint/UI_scene.UI_scene_C"))
      (Variables|/Game/Dance_anim_content/Blueprint/UI_scene.UI_scene_C|SetDancer_actor _returnvalue self)
      (UserInterface|Viewport|AddtoViewport _returnvalue 0))
    (:then_1
      ;[0.2608 1 0] Event to change dance
      (Default|ChangeMode (.AsDance (Utilities|Casting|CastToDance (Components|SkeletalMesh|GetAnimInstance (Variables|/Script/Engine.Character|GetMesh self)))) (Variables|Default|GetDance_type)))))

(fn ConstructionScript)